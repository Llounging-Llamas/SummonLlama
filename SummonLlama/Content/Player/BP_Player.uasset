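; Player character for a potion-brewing game, handling Enhanced Input movement, a journal widget and two-handed ingredient carrying.
; Each hand picks up overlapping BPI_Interact actors or respawns its held item; held spoon and knife flags gate cauldron stirring and chopping.
; The summon input drives chopping, cauldron summoning and mortar use, with ingredients transformed by swapping type and mesh.
; Death shrinks the player into a rat until Y reloads the level.
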(event `EnhancedInput|/Game/Input/Actions/IA_Movement`
  (params (ActionValue :type "Vector2D Structure") (ElapsedSeconds :type "Float (double-precision)") (TriggeredSeconds :type "Float (double-precision)") (InputAction :type "InputAction Object Reference" :default "/Game/Input/Actions/IA_Movement.IA_Movement"))
  (bind (_returnvalue_roll _returnvalue_pitch _returnvalue_yaw) (`KismetMathLibrary.BreakRotator` (`self.GetControlRotation`)))
  ;[1 1 1] Input
  ;;[1 1 1] Player Movement Input
  (:`Triggered`
    (`self.AddMovementInput` (`KismetMathLibrary.GetRightVector` (`self.GetControlRotation`)) ActionValue_X)
    (`self.AddMovementInput` (`KismetMathLibrary.GetForwardVector` (`KismetMathLibrary.MakeRotator` _returnvalue_roll 0.0 _returnvalue_yaw)) ActionValue_Y)))

(event `EnhancedInput|/Game/Input/Actions/IA_LookAround`
  (params (ActionValue :type "Vector2D Structure") (ElapsedSeconds :type "Float (double-precision)") (TriggeredSeconds :type "Float (double-precision)") (InputAction :type "InputAction Object Reference" :default "/Game/Input/Actions/IA_LookAround.IA_LookAround"))
  ;[1 1 1] Input
  ;;[1 1 1] Player Movement Input
  (:`Triggered`
    (`self.AddControllerYawInput` ActionValue_X)
    (`self.AddControllerPitchInput` ActionValue_Y)))

(event `self.ReceiveBeginPlay`
  (bind _returnvalue (pcsubsystem `EnhancedInputLocalPlayerSubsystem` (`GameplayStatics.GetPlayerController` 0)))
  (`/Engine/EditorBlueprintResources/StandardMacros.IsValid` _returnvalue
    (:`Is Valid`
      (`EnhancedInputSubsystemInterface.AddMappingContext` _returnvalue "/Game/Input/IMC_Player.IMC_Player" 0 (struct))
      (bind _returnvalue_2 (`|CreateWidget` "/Game/UI/P_NoKnife.P_NoKnife_C"))
      (set `self.PromptNoKnife` _returnvalue_2))))

(event `EnhancedInput|/Game/Input/Actions/IA_InteractLeft`
  (params (ActionValue :type Boolean) (ElapsedSeconds :type "Float (double-precision)") (TriggeredSeconds :type "Float (double-precision)") (InputAction :type "InputAction Object Reference" :default "/Game/Input/Actions/IA_InteractLeft.IA_InteractLeft"))
  ;[1 1 1] Input
  ;;[1 1 1] Left hand interact + pick up and drop items
  (:`Triggered`
    (if (`self.IsAtCauldron`)
      (if (`self.HasSpoon`)
        (`self.StirCauldronClockwise`)
        (else
          (if (`self.HasLeftItem`) :!label _label
            (bind _returnvalue (`|SpawnActorFromClass` (`GameplayStatics.GetObjectClass` (`self.LeftItem`)) (`KismetMathLibrary.MakeTransform` (`SceneComponent.GetSocketLocation` (`self.Item_Left`) "None")) "Undefined" "MultiplyWithRoot" null null))
            (message `/Game/Objects/Ingredients/BPI_Ingredients.SetIngredientMesh` _returnvalue (`StaticMeshComponent.StaticMesh` (`self.Item_Left`)) (`PrimitiveComponent.GetMaterial` (`self.Item_Left`) 0))
            (message `/Game/Objects/Ingredients/BPI_Ingredients.SetIngredientType` _returnvalue (`self.LeftItemType`))
            (`StaticMeshComponent.SetStaticMesh` (`self.Item_Left`) null)
            (`PrimitiveComponent.SetMaterial` (`self.Item_Left`) 0 null)
            (set `self.HasLeftItem` false)
            (`self.CheckIfSpoon`)
            (`self.CheckIfKnife`)
            (`KismetSystemLibrary.PrintString` "spawned in dropped item")
            (else
              (for _array_element (`self.GetOverlappingActors` "/Script/Engine.Actor")
                (if (`KismetSystemLibrary.DoesImplementInterface` _array_element "/Game/Objects/BPI_Interact.BPI_Interact_C")
                  (message `/Game/Objects/BPI_Interact.Interact` _array_element)
                  (`StaticMeshComponent.SetStaticMesh` (`self.Item_Left`) (`self.PickedUpItemMesh`))
                  (`PrimitiveComponent.SetMaterial` (`self.Item_Left`) 0 (`self.PickedUpItemMaterial`))
                  (`PrimitiveComponent.SetMaterial` (`self.Item_Left`) 1 (`self.PickedUpItemMaterial`))
                  (set `self.LeftItem` (`self.PickedUpItem`))
                  (set `self.HasLeftItem` true)
                  (set `self.LeftItemType` (`self.PickedUpItemType`))
                  (break)))))))
      (else
        (goto _label)))))

(event `ProcessChopping`
  (bind _item_right (`self.Item_Right`))
  (bind _item_left (`self.Item_Left`))
  (bind _promptnoknife (`self.PromptNoKnife`))
  ;[1 1 1] Chopping with knife and chopping block object -> will chop a finger if the player has a knife and no ingredient (on E press)
  (if (`self.IsAtChoppingBoard`)
    (if (`self.HasKnife`)
      (if (`self.HasRightItem`)
        (if (`self.HasLeftItem`)
          (if (== (`StaticMeshComponent.StaticMesh` (`self.Item_Left`)) "/ControlRig/Controls/ControlRig_Line.ControlRig_Line")
            (switch `/Game/Objects/Ingredients/E_IngredientType` (`self.RightItemType`)
              (:`NewEnumerator0`
                (set `self.LeftItemType` "NewEnumerator6")
                (`StaticMeshComponent.SetStaticMesh` _item_right "/Game/Props/Obj_Carrot_Chopped.Obj_Carrot_Chopped")
                (`KismetSystemLibrary.PrintString` "ingredient chopped" :!label _label_2))
              (:`NewEnumerator1`
                (set `self.LeftItemType` "NewEnumerator7")
                (`StaticMeshComponent.SetStaticMesh` _item_right "/Game/Props/Obj_Eye_Chopped.Obj_Eye_Chopped")
                (goto _label_2))
              (:`NewEnumerator2`
                (`KismetSystemLibrary.PrintString` "other ingredient type" :!label _label_3))
              (:`NewEnumerator3`
                (goto _label_3))
              (:`NewEnumerator4`
                (goto _label_3))
              (:`NewEnumerator5`
                (goto _label_3))
              (:`NewEnumerator6`
                (goto _label_3))
              (:`NewEnumerator7`
                (goto _label_3))
              (:`NewEnumerator8`
                (goto _label_3))
              (:`NewEnumerator9`
                (goto _label_3))
              (:`NewEnumerator10`
                (goto _label_3))
              (:`NewEnumerator11`
                (goto _label_3)))
            (else
              (switch `/Game/Objects/Ingredients/E_IngredientType` (`self.LeftItemType`)
                (:`NewEnumerator0`
                  (set `self.LeftItemType` "NewEnumerator6")
                  (`StaticMeshComponent.SetStaticMesh` _item_left "/Game/Props/Obj_Carrot_Chopped.Obj_Carrot_Chopped")
                  (`KismetSystemLibrary.PrintString` "ingredient chopped" :!label _label_4))
                (:`NewEnumerator1`
                  (set `self.LeftItemType` "NewEnumerator7")
                  (`StaticMeshComponent.SetStaticMesh` _item_left "/Game/Props/Obj_Eye_Chopped.Obj_Eye_Chopped")
                  (goto _label_4))
                (:`NewEnumerator2`
                  (`KismetSystemLibrary.PrintString` "other ingredient type" :!label _label_5))
                (:`NewEnumerator3`
                  (goto _label_5))
                (:`NewEnumerator4`
                  (goto _label_5))
                (:`NewEnumerator5`
                  (goto _label_5))
                (:`NewEnumerator6`
                  (goto _label_5))
                (:`NewEnumerator7`
                  (goto _label_5))
                (:`NewEnumerator8`
                  (goto _label_5))
                (:`NewEnumerator9`
                  (goto _label_5))
                (:`NewEnumerator10`
                  (goto _label_5))
                (:`NewEnumerator11`
                  (goto _label_5)))))
          (else
            (`|SpawnActorFromClass` "/Game/Objects/Ingredients/BP_IngredientFinger.BP_IngredientFinger_C" (`KismetMathLibrary.MakeTransform` (`SceneComponent.GetSocketLocation` (`self.Item_Left`) "None")) "Undefined" "MultiplyWithRoot" null null)
            (`KismetSystemLibrary.PrintString` "chop and spawn" :!label _label_6)))
        (elif (`self.HasLeftItem`)
          (`|SpawnActorFromClass` "/Game/Objects/Ingredients/BP_IngredientFinger.BP_IngredientFinger_C" (`KismetMathLibrary.MakeTransform` (`SceneComponent.GetSocketLocation` (`self.Item_Right`) "None")) "Undefined" "MultiplyWithRoot" null null)
          (goto _label_6)
          (else
            (`KismetSystemLibrary.PrintString` "no held items registered"))))
      (else
        (`UserWidget.AddToViewport` _promptnoknife 0)
        (`KismetSystemLibrary.PrintString` "no knife")
        (`KismetSystemLibrary.Delay` 2.0)
        (`Widget.RemoveFromParent` _promptnoknife)))
    (else
      (`KismetSystemLibrary.PrintString` "not at chopping block"))))

(event `EnhancedInput|/Game/Input/Actions/IA_InteractRight`
  (params (ActionValue :type Boolean) (ElapsedSeconds :type "Float (double-precision)") (TriggeredSeconds :type "Float (double-precision)") (InputAction :type "InputAction Object Reference" :default "/Game/Input/Actions/IA_InteractRight.IA_InteractRight"))
  ;[1 1 1] Input
  ;;[1 1 1] Right hand interact + pick up and drop items
  (:`Triggered`
    (if (`self.IsAtCauldron`)
      (if (`self.HasSpoon`)
        (`self.StirCauldronAnticlockwise`)
        (else
          (if (`self.HasRightItem`) :!label _label_7
            (bind _returnvalue (`|SpawnActorFromClass` (`GameplayStatics.GetObjectClass` (`self.RightItem`)) (`KismetMathLibrary.MakeTransform` (`SceneComponent.GetSocketLocation` (`self.Item_Right`) "None")) "Undefined" "MultiplyWithRoot" null null))
            (message `/Game/Objects/Ingredients/BPI_Ingredients.SetIngredientMesh` _returnvalue (`StaticMeshComponent.StaticMesh` (`self.Item_Right`)) (`PrimitiveComponent.GetMaterial` (`self.Item_Right`) 0))
            (message `/Game/Objects/Ingredients/BPI_Ingredients.SetIngredientType` _returnvalue (`self.RightItemType`))
            (`StaticMeshComponent.SetStaticMesh` (`self.Item_Right`) null)
            (`PrimitiveComponent.SetMaterial` (`self.Item_Right`) 0 null)
            (set `self.HasRightItem` false)
            (`self.CheckIfSpoon`)
            (`self.CheckIfKnife`)
            (`KismetSystemLibrary.PrintString` "spawned in dropped item")
            (else
              (for _array_element (`self.GetOverlappingActors` "/Script/Engine.Actor")
                (if (`KismetSystemLibrary.DoesImplementInterface` _array_element "/Game/Objects/BPI_Interact.BPI_Interact_C")
                  (message `/Game/Objects/BPI_Interact.Interact` _array_element)
                  (`StaticMeshComponent.SetStaticMesh` (`self.Item_Right`) (`self.PickedUpItemMesh`))
                  (`PrimitiveComponent.SetMaterial` (`self.Item_Right`) 0 (`self.PickedUpItemMaterial`))
                  (`PrimitiveComponent.SetMaterial` (`self.Item_Right`) 1 (`self.PickedUpItemMaterial`))
                  (set `self.RightItem` (`self.PickedUpItem`))
                  (set `self.HasRightItem` true)
                  (set `self.RightItemType` (`self.PickedUpItemType`))
                  (break)))))))
      (else
        (goto _label_7)))))

(event `EnhancedInput|/Game/Input/Actions/IA_Journal`
  (params (ActionValue :type Boolean) (ElapsedSeconds :type "Float (double-precision)") (TriggeredSeconds :type "Float (double-precision)") (InputAction :type "InputAction Object Reference" :default "/Game/Input/Actions/IA_Journal.IA_Journal"))
  (bind _returnvalue (`GameplayStatics.GetPlayerController` 0))
  ;[1 1 1] Journal
  (:`Started`
    (bind _returnvalue_2 (`|CreateWidget` "/Game/UI/Journal.Journal_C"))
    (`UserWidget.AddToViewport` _returnvalue_2 0)
    (set `PlayerController.bShowMouseCursor` true _returnvalue)
    (`WidgetBlueprintLibrary.SetInputMode_UIOnlyEx` _returnvalue null)))

(event `CheckIfSpoon`
  ;[1 1 1] Updates if player is holding a spoon
  (if (== (`self.LeftItem`) "/Game/Objects/BP_StirringSpoon.BP_StirringSpoon")
    (if (`self.HasLeftItem`)
      (set `self.HasSpoon` true :!label _label_8))
    (elif (== (`self.RightItem`) "/Game/Objects/BP_StirringSpoon.BP_StirringSpoon")
      (if (`self.HasRightItem`)
        (goto _label_8))
      (else
        (set `self.HasSpoon` false)))))

(event `CheckIfKnife`
  ;[1 1 1] Updates if player is holding a knife
  (if (== (`StaticMeshComponent.StaticMesh` (`self.Item_Left`)) "/ControlRig/Controls/ControlRig_Line.ControlRig_Line")
    (if (`self.HasLeftItem`)
      (set `self.HasKnife` true :!label _label_9))
    (elif (== (`StaticMeshComponent.StaticMesh` (`self.Item_Right`)) "/ControlRig/Controls/ControlRig_Line.ControlRig_Line")
      (if (`self.HasRightItem`)
        (goto _label_9))
      (else
        (set `self.HasKnife` false)))))

(event `UseMortarAndPestle`
  ;[1 1 1] Mortar and pestle main functionality
  (for _array_element (`self.GetOverlappingActors` "/Script/Engine.Actor")
    (cast `/Game/Objects/BP_MortarAndPestle` _array_element
      (:`then`
        (if (`self.HasLeftItem`)
          (if (`self.HasRightItem`)
            (`KismetSystemLibrary.PrintString` "Failed - has 2 items")
            (elif (`self.HasSpoon`)
              (`KismetSystemLibrary.PrintString` "Failed - has left spoon")
              (else
                (switch `/Game/Objects/Ingredients/E_IngredientType` (`self.LeftItemType`)
                  (:`NewEnumerator0`
                    (set `self.LeftItemType` "NewEnumerator9")
                    (`StaticMeshComponent.SetStaticMesh` (`self.Item_Left`) "/ControlRig/Controls/ControlRig_Diamond_3mm.ControlRig_Diamond_3mm" :!label _label_10)
                    (`KismetSystemLibrary.PrintString` "Player UseMortarAndPestle completed")
                    (break))
                  (:`NewEnumerator1`
                    (set `self.LeftItemType` "NewEnumerator10")
                    (goto _label_10))
                  (:`NewEnumerator2`
                    (set `self.LeftItemType` "NewEnumerator11")
                    (goto _label_10))
                  (:`NewEnumerator3`
                    _)
                  (:`NewEnumerator4`
                    _)
                  (:`NewEnumerator5`
                    _)
                  (:`NewEnumerator6`
                    _)
                  (:`NewEnumerator7`
                    _)
                  (:`NewEnumerator8`
                    _)
                  (:`NewEnumerator9`
                    _)
                  (:`NewEnumerator10`
                    _)
                  (:`NewEnumerator11`
                    _))
                (`KismetSystemLibrary.PrintString` "other ingredient type"))))
          (elif (`self.HasRightItem`)
            (if (`self.HasSpoon`)
              (`KismetSystemLibrary.PrintString` "Failed - has right spoon")
              (else
                (switch `/Game/Objects/Ingredients/E_IngredientType` (`self.RightItemType`)
                  (:`NewEnumerator0`
                    (set `self.RightItemType` "NewEnumerator9")
                    (`StaticMeshComponent.SetStaticMesh` (`self.Item_Right`) "/ControlRig/Controls/ControlRig_Diamond_3mm.ControlRig_Diamond_3mm" :!label _label_11)
                    (`KismetSystemLibrary.PrintString` "Player UseMortarAndPestle completed")
                    (break))
                  (:`NewEnumerator1`
                    (set `self.RightItemType` "NewEnumerator10")
                    (goto _label_11))
                  (:`NewEnumerator2`
                    (set `self.RightItemType` "NewEnumerator11")
                    (goto _label_11))
                  (:`NewEnumerator3`
                    _)
                  (:`NewEnumerator4`
                    _)
                  (:`NewEnumerator5`
                    _)
                  (:`NewEnumerator6`
                    _)
                  (:`NewEnumerator7`
                    _)
                  (:`NewEnumerator8`
                    _)
                  (:`NewEnumerator9`
                    _)
                  (:`NewEnumerator10`
                    _)
                  (:`NewEnumerator11`
                    _))
                (`KismetSystemLibrary.PrintString` "other ingredient type")))
            (else
              (`KismetSystemLibrary.PrintString` "Failed - has no items")))))
      (:`CastFailed`
        (`KismetSystemLibrary.PrintString` "No Mortar and Pestle")))))

(event `StirCauldronClockwise`
  ;[1 1 1] Cauldron stir cloclwise
  (for _array_element (`self.GetOverlappingActors` "/Script/Engine.Actor")
    (bind _asbp_cauldron (cast `/Game/Objects/BP_Cauldron` _array_element))
    (set `/Game/Objects/BP_Cauldron.IsClockwiseStirred` true _asbp_cauldron)
    (`KismetSystemLibrary.PrintString` "stirred clockwise")
    (break)))

(event `StirCauldronAnticlockwise`
  ;[1 1 1] Cauldron stir anticlockwise
  (for _array_element (`self.GetOverlappingActors` "/Script/Engine.Actor")
    (bind _asbp_cauldron (cast `/Game/Objects/BP_Cauldron` _array_element))
    (set `/Game/Objects/BP_Cauldron.IsAnticlockwiseStirred` true _asbp_cauldron)
    (`KismetSystemLibrary.PrintString` "stirred anticlockwise")
    (break)))

(event `EnhancedInput|/Game/Input/Actions/IA_Summon`
  (params (ActionValue :type Boolean) (ElapsedSeconds :type "Float (double-precision)") (TriggeredSeconds :type "Float (double-precision)") (InputAction :type "InputAction Object Reference" :default "/Game/Input/Actions/IA_Summon.IA_Summon"))
  ;[1 1 1] Summon on E press when overlapping the cauldron
  (:`Triggered`
    (`self.ProcessChopping`)
    (for _array_element (`self.GetOverlappingActors` "/Script/Engine.Actor")
      (`|ExecutionSequence`
        (:`then_0`
          (bind _asbp_cauldron (cast `/Game/Objects/BP_Cauldron` _array_element))
          (`/Game/Objects/BP_Cauldron.Summon` _asbp_cauldron)
          (break))
        (:`then_1`
          (bind _asbp_mortar_and_pestle (cast `/Game/Objects/BP_MortarAndPestle` _array_element))
          (`/Game/Objects/BP_MortarAndPestle.Use` _asbp_mortar_and_pestle))))))

(event `EnhancedInput|/Game/Input/Actions/IA_CleanCauldron`
  (params (ActionValue :type Boolean) (ElapsedSeconds :type "Float (double-precision)") (TriggeredSeconds :type "Float (double-precision)") (InputAction :type "InputAction Object Reference" :default "/Game/Input/Actions/IA_CleanCauldron.IA_CleanCauldron"))
  ;[1 1 1] Clean Cauldron on C press
  (:`Triggered`
    (for _array_element (`self.GetOverlappingActors` "/Script/Engine.Actor")
      (bind _asbp_cauldron (cast `/Game/Objects/BP_Cauldron` _array_element))
      (`/Game/Objects/BP_Cauldron.CleanCauldron` _asbp_cauldron)
      (break))))

(event `DEATH!`
  ;[1 1 1] TURNED INTO A RAT! Function
  (set `self.israt` true)
  (bind _returnvalue (`|CreateWidget` "/Game/UI/WB_RATWidget.WB_RATWidget_C"))
  (`UserWidget.AddToViewport` _returnvalue 0)
  (`self.SetActorScale3D` (`GameplayStatics.GetPlayerCharacter` 0) (0.1 0.1 0.1)))

(event `Key|Y`
  (params (Key :type "Key Structure"))
  ;[1 1 1] TURNED INTO A RAT! Function
  (:`Pressed`
    (if (`self.israt`)
      (set `self.israt` false)
      (`GameplayStatics.OpenLevel` "Finnmap"))))

(fn `UserConstructionScript`)