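; Game instance for a cooking game that holds the recipe progression, patience meter and moon state.
; Events raise or lower patience, and the small-step drain calls DEATH on the player character once it reaches zero.
; A correct recipe advances the recipe enum and plays delayed Devil voice lines announcing the next dish, or shows the win screen after the last.
; Moon visibility is off for the first recipe and random afterwards.
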(event `DecreasePatience20%`
  (set `self.PatiencePercent` (- (`self.PatiencePercent`) 0.2)))

(event `increasepatienceby20%`
  (set `self.PatiencePercent` (+ (`self.PatiencePercent`) 0.2)))

(event `DecreasePatienceBysmall amount`
  (set `self.PatiencePercent` (- (`self.PatiencePercent`) 0.004))
  (if (<= (`self.PatiencePercent`) 0.0)
    (`/Engine/EditorBlueprintResources/StandardMacros.DoOnce` false
      (:`Completed`
        (bind _asbp_player (cast `/Game/Player/BP_Player` (`GameplayStatics.GetPlayerCharacter` 0)))
        (`/Game/Player/BP_Player.DEATH!` _asbp_player)))))

(event `ProcessCorrectRecipe`
  (if (<= (`self.CurrentRecipe`) 8)
    (set `self.IsRecipeCorrect` false)
    (set `self.CurrentRecipe` (cast `/Game/Recipes/ERecipes` (+ (`self.CurrentRecipe`) 1)))
    (`KismetSystemLibrary.Delay` 9.0)
    (`GameplayStatics.PlaySound2D` "/Game/Sounds/devil_make_me___.devil_make_me___" 1.0 1.0 0.0 null null)
    (`KismetSystemLibrary.Delay` 2.0)
    (switch `int` (`KismetMathLibrary.Conv_ByteToInt` (`self.CurrentRecipe`))
      (:`1`
        (`KismetSystemLibrary.PrintString` "SECCCCCCCCCCCCCCCCCCCCCCCCCCCCCCCCCCCCCCCCCCCCCCCCCCCCCCCCOND RECIPE")
        (`GameplayStatics.PlaySound2D` "/Game/Sounds/devil_sinful_shadow_gumbo.devil_sinful_shadow_gumbo" 1.0 1.0 0.0 null null))
      (:`2`
        (`GameplayStatics.PlaySound2D` "/Game/Sounds/devil_infernal_eruption_pasta.devil_infernal_eruption_pasta" 1.0 1.0 0.0 null null))
      (:`3`
        (`GameplayStatics.PlaySound2D` "/Game/Sounds/devil_brimstone_bbq_skewers.devil_brimstone_bbq_skewers" 1.0 1.0 0.0 null null))
      (:`4`
        (`GameplayStatics.PlaySound2D` "/Game/Sounds/sinister_serpent_stew.sinister_serpent_stew" 1.0 1.0 0.0 null null))
      (:`5`
        (`GameplayStatics.PlaySound2D` "/Game/Sounds/devil_lucifer_s_lava_linguine.devil_lucifer_s_lava_linguine" 1.0 1.0 0.0 null null))
      (:`6`
        (`GameplayStatics.PlaySound2D` "/Game/Sounds/devil_demonic_delight_curry.devil_demonic_delight_curry" 1.0 1.0 0.0 null null))
      (:`7`
        (`GameplayStatics.PlaySound2D` "/Game/Sounds/devil_malignant_moonlight_macaroni.devil_malignant_moonlight_macaroni" 1.0 1.0 0.0 null null))
      (:`8`
        (`GameplayStatics.PlaySound2D` "/Game/Sounds/devil_hellhound_hash_browns.devil_hellhound_hash_browns" 1.0 1.0 0.0 null null)))
    (else
      (bind _returnvalue (`|CreateWidget` "/Game/UI/WB_WinScreen.WB_WinScreen_C"))
      (`UserWidget.AddToViewport` _returnvalue 0))))

(event `UpdateMoonState`
  (switch `/Game/Recipes/ERecipes` (`self.CurrentRecipe`)
    (:`NewEnumerator0`
      (set `self.IsMoonVisible` false))
    (:`NewEnumerator1`
      (set `self.IsMoonVisible` (`KismetMathLibrary.RandomBool`) :!label _label))
    (:`NewEnumerator2`
      (goto _label))
    (:`NewEnumerator3`
      (goto _label))
    (:`NewEnumerator4`
      (goto _label))
    (:`NewEnumerator5`
      (goto _label))
    (:`NewEnumerator6`
      (goto _label))
    (:`NewEnumerator7`
      (goto _label))
    (:`NewEnumerator8`
      (goto _label))
    (:`NewEnumerator9`
      (goto _label))))