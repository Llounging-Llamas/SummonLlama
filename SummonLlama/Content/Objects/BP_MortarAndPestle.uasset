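; BP_MortarAndPestle is an interactable mortar and pestle object that the player can use when nearby.
; On BeginPlay it creates a P_Mortar prompt widget, which overlaps with its CollisionSphere or Box show and hide for the player.
; Only the sphere also toggles the player's IsAtMortarAndPestle flag.
; Its Use event hands the action to BP_Player's UseMortarAndPestle and prints a debug message.
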(event `Use`
  (bind _asbp_player (cast `/Game/Player/BP_Player` (`GameplayStatics.GetPlayerCharacter` 0)))
  (`/Game/Player/BP_Player.UseMortarAndPestle` _asbp_player)
  (`KismetSystemLibrary.PrintString` "BP_MortarAndPestle Activated"))

(event `self.ReceiveBeginPlay`
  (bind _returnvalue (`|CreateWidget` "/Game/UI/P_Mortar.P_Mortar_C"))
  (set `self.Mortar Prompt` _returnvalue))

(event `self.CollisionSphere.OnComponentBeginOverlap`
  (params (OverlappedComponent :type "PrimitiveComponent Object Reference") (OtherActor :type "Actor Object Reference") (OtherComp :type "PrimitiveComponent Object Reference") (OtherBodyIndex :type Integer) (bFromSweep :type Boolean) (SweepResult :type "HitResult Structure (by ref)"))
  (if (== OtherActor (`GameplayStatics.GetPlayerCharacter` 0))
    (`UserWidget.AddToViewport` (`self.Mortar Prompt`) 0)
    (bind _asbp_player (cast `/Game/Player/BP_Player` OtherActor))
    (set `/Game/Player/BP_Player.IsAtMortarAndPestle` true _asbp_player)))

(event `self.CollisionSphere.OnComponentEndOverlap`
  (params (OverlappedComponent :type "PrimitiveComponent Object Reference") (OtherActor :type "Actor Object Reference") (OtherComp :type "PrimitiveComponent Object Reference") (OtherBodyIndex :type Integer))
  (if (== (`GameplayStatics.GetPlayerCharacter` 0) OtherActor)
    (`Widget.RemoveFromParent` (`self.Mortar Prompt`))
    (bind _asbp_player (cast `/Game/Player/BP_Player` OtherActor))
    (set `/Game/Player/BP_Player.IsAtMortarAndPestle` false _asbp_player)))

(event `self.Box.OnComponentBeginOverlap`
  (params (OverlappedComponent :type "PrimitiveComponent Object Reference") (OtherActor :type "Actor Object Reference") (OtherComp :type "PrimitiveComponent Object Reference") (OtherBodyIndex :type Integer) (bFromSweep :type Boolean) (SweepResult :type "HitResult Structure (by ref)"))
  (if (== OtherActor (`GameplayStatics.GetPlayerCharacter` 0))
    (`UserWidget.AddToViewport` (`self.Mortar Prompt`) 0)))

(event `self.Box.OnComponentEndOverlap`
  (params (OverlappedComponent :type "PrimitiveComponent Object Reference") (OtherActor :type "Actor Object Reference") (OtherComp :type "PrimitiveComponent Object Reference") (OtherBodyIndex :type Integer))
  (if (== (`GameplayStatics.GetPlayerCharacter` 0) OtherActor)
    (`Widget.RemoveFromParent` (`self.Mortar Prompt`))))

(fn `UserConstructionScript`)