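; Carrot ingredient actor that the player can pick up and that can be charred, chopped or crushed.
; Each state change sets the type enum and refreshes the mesh, reusing the carrot mesh with a different material per processed state.
; Interact passes the mesh and a self reference to BP_Player, then destroys the actor after a tiny delay.
; Any overlap on the mesh sets SummonType to the carrot's hard-coded value in FinnGameInstance.
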(event `self.ReceiveBeginPlay`
  (`self.SetIngredientMesh`))

(event `self.StaticMesh.OnComponentBeginOverlap`
  (params (OverlappedComponent :type "PrimitiveComponent Object Reference") (OtherActor :type "Actor Object Reference") (OtherComp :type "PrimitiveComponent Object Reference") (OtherBodyIndex :type Integer) (bFromSweep :type Boolean) (SweepResult :type "HitResult Structure (by ref)"))
  (bind _asfinn_game_instance (cast `/Game/Blueprints/FinnGameInstance` (`GameplayStatics.GetGameInstance`)))
  (bind _output_get (set `/Game/Blueprints/FinnGameInstance.SummonType` 3 _asfinn_game_instance))
  (`KismetSystemLibrary.PrintString` (`KismetStringLibrary.Conv_IntToString` _output_get)))

(event `/Game/Objects/BPI_Interact.Interact`
  ;[1 1 1] Pick up the ingredient
  (bind _asbp_player (cast `/Game/Player/BP_Player` (`GameplayStatics.GetPlayerCharacter` 0)))
  (set `/Game/Player/BP_Player.PickedUpItemMesh` "/Game/Props/Obj_Carrot.Obj_Carrot" _asbp_player)
  (set `/Game/Player/BP_Player.PickedUpItem` self _asbp_player)
  (`KismetSystemLibrary.Delay` 0.01)
  (`self.K2_DestroyActor`)
  (`KismetSystemLibrary.PrintString` "Item Picked Up"))

(event `/Game/Objects/Ingredients/BPI_Ingredients.CharIngredient`
  ;[1 1 1] Change the ingredient state
  (set `self.Type` "NewEnumerator3")
  (`self.SetIngredientMesh` :!label _label))

(event `SetIngredientMesh`
  (bind _staticmesh (`self.StaticMesh`))
  ;[1 1 1] Updates the mesh/material of the ingredient based on its type
  (switch `/Game/Objects/Ingredients/E_IngredientType` (`self.Type`)
    (:`NewEnumerator0`
      (`StaticMeshComponent.SetStaticMesh` _staticmesh "/Game/Props/Obj_Carrot.Obj_Carrot"))
    (:`NewEnumerator3`
      (`StaticMeshComponent.SetStaticMesh` _staticmesh "/Game/Props/Obj_Carrot.Obj_Carrot")
      (`PrimitiveComponent.SetMaterial` _staticmesh 0 "/AnimationSharing/AnimSharingRed.AnimSharingRed"))
    (:`NewEnumerator6`
      (`StaticMeshComponent.SetStaticMesh` _staticmesh "/Game/Props/Obj_Carrot.Obj_Carrot")
      (`PrimitiveComponent.SetMaterial` _staticmesh 0 "/AnimationSharing/AnimSharingGreen.AnimSharingGreen"))
    (:`NewEnumerator9`
      (`StaticMeshComponent.SetStaticMesh` _staticmesh "/Game/Props/Obj_Carrot.Obj_Carrot")
      (`PrimitiveComponent.SetMaterial` _staticmesh 0 "/Engine/VREditor/UI/ArrowMaterial.ArrowMaterial"))))

(event `/Game/Objects/Ingredients/BPI_Ingredients.ChopIngredient`
  ;[1 1 1] Change the ingredient state
  (set `self.Type` "NewEnumerator6")
  (goto _label))

(event `/Game/Objects/Ingredients/BPI_Ingredients.CrushIngredient`
  ;[1 1 1] Change the ingredient state
  (set `self.Type` "NewEnumerator9")
  (goto _label))

(fn `GetIngredientType`
  (returns (IngredientType :type "/Game/Objects/Ingredients/E_IngredientType Enum"))
  (return (`self.Type`)))

(fn `UserConstructionScript`)