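; BP_IngredientEye is a pickup eye ingredient that carries a type state which processing can change.
; Interact copies its mesh, material, type and self reference to BP_Player, then destroys it if it sits below a height threshold.
; Char, Chop and Crush events switch the type, with charring also swapping the mesh and materials, and setters allow external overrides.
; Overlapping the mesh sets SummonType on FinnGameInstance, and debug prints report state.
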(event `self.ReceiveBeginPlay`
  ;[1 1 1] Just checking spawned items with state changes work
  (`KismetSystemLibrary.DelayUntilNextTick`)
  (`KismetSystemLibrary.PrintString` (`|GetEnumeratorNameAsString` (`self.Type`)))
  (`KismetSystemLibrary.PrintString` "Obj Type"))

(event `self.StaticMesh.OnComponentBeginOverlap`
  (params (OverlappedComponent :type "PrimitiveComponent Object Reference") (OtherActor :type "Actor Object Reference") (OtherComp :type "PrimitiveComponent Object Reference") (OtherBodyIndex :type Integer) (bFromSweep :type Boolean) (SweepResult :type "HitResult Structure (by ref)"))
  (bind _asfinn_game_instance (cast `/Game/Blueprints/FinnGameInstance` (`GameplayStatics.GetGameInstance`)))
  (bind _output_get (set `/Game/Blueprints/FinnGameInstance.SummonType` 1 _asfinn_game_instance))
  (`KismetSystemLibrary.PrintString` (`KismetStringLibrary.Conv_IntToString` _output_get)))

(event `/Game/Objects/BPI_Interact.Interact`
  (bind (_returnvalue_x _returnvalue_y _returnvalue_z) (`KismetMathLibrary.BreakVector` (`SceneComponent.K2_GetComponentLocation` (`self.DefaultSceneRoot`))))
  ;[1 1 1] Pick up the ingredient
  (bind _asbp_player (cast `/Game/Player/BP_Player` (`GameplayStatics.GetPlayerCharacter` 0)))
  (set `/Game/Player/BP_Player.PickedUpItemMesh` (`StaticMeshComponent.StaticMesh` (`self.StaticMesh`)) _asbp_player)
  (set `/Game/Player/BP_Player.PickedUpItemMaterial` (`PrimitiveComponent.GetMaterial` (`self.StaticMesh`) 0) _asbp_player)
  (set `/Game/Player/BP_Player.PickedUpItem` self _asbp_player)
  (set `/Game/Player/BP_Player.PickedUpItemType` (`self.Type`) _asbp_player)
  (if (< _returnvalue_z 149.0)
    (`KismetSystemLibrary.Delay` 0.01)
    (`self.K2_DestroyActor`)
    (`KismetSystemLibrary.PrintString` "Item Picked Up")))

(event `/Game/Objects/Ingredients/BPI_Ingredients.CharIngredient`
  ;[1 1 1] Change the ingredient state
  (set `self.Type` "NewEnumerator4")
  (`StaticMeshComponent.SetStaticMesh` (`self.StaticMesh`) "/Game/Props/Obj_Eye.Obj_Eye")
  (`PrimitiveComponent.SetMaterial` (`self.StaticMesh`) 0 "/AnimationSharing/AnimSharingRed.AnimSharingRed")
  (`PrimitiveComponent.SetMaterial` (`self.StaticMesh`) 1 "/AnimationSharing/AnimSharingRed.AnimSharingRed"))

(event `/Game/Objects/Ingredients/BPI_Ingredients.ChopIngredient`
  ;[1 1 1] Change the ingredient state
  (set `self.Type` "NewEnumerator7"))

(event `/Game/Objects/Ingredients/BPI_Ingredients.CrushIngredient`
  ;[1 1 1] Change the ingredient state
  (set `self.Type` "NewEnumerator10"))

(event `/Game/Objects/Ingredients/BPI_Ingredients.SetIngredientMesh`
  (params (Mesh :type "StaticMesh Object Reference") (Material :type "MaterialInterface Object Reference"))
  (`StaticMeshComponent.SetStaticMesh` (`self.StaticMesh`) Mesh)
  (`PrimitiveComponent.SetMaterial` (`self.StaticMesh`) 0 Material)
  (`PrimitiveComponent.SetMaterial` (`self.StaticMesh`) 1 Material))

(event `/Game/Objects/Ingredients/BPI_Ingredients.SetIngredientType`
  (params (Type :type "/Game/Objects/Ingredients/E_IngredientType Enum" :default "NewEnumerator0"))
  (set `self.Type` Type))

(fn `GetIngredientType`
  (returns (IngredientType :type "/Game/Objects/Ingredients/E_IngredientType Enum"))
  (return (`self.Type`)))

(fn `UserConstructionScript`)