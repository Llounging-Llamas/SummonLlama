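; Cauldron actor where the player drops ingredients in order to brew demon-summoning recipes.
; It spawns the GameInstance's current recipe actor and reads three required ingredients from it.
; Overlapping BPI_Ingredients items are recorded and destroyed, then compared in exact order to set IsRecipeCorrect.
; Externally triggered events handle summoning, success or goopey-demon failure, and cleaning the dirty cauldron, which blocks correct brews until cleaned.
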(event `self.Box.OnComponentEndOverlap`
  (params (OverlappedComponent :type "PrimitiveComponent Object Reference") (OtherActor :type "Actor Object Reference") (OtherComp :type "PrimitiveComponent Object Reference") (OtherBodyIndex :type Integer))
  (bind _asbp_player (cast `/Game/Player/BP_Player` OtherActor))
  (set `/Game/Player/BP_Player.IsAtCauldron` false _asbp_player))

(event `self.Box.OnComponentBeginOverlap`
  (params (OverlappedComponent :type "PrimitiveComponent Object Reference") (OtherActor :type "Actor Object Reference") (OtherComp :type "PrimitiveComponent Object Reference") (OtherBodyIndex :type Integer) (bFromSweep :type Boolean) (SweepResult :type "HitResult Structure (by ref)"))
  (bind _asbp_player (cast `/Game/Player/BP_Player` OtherActor)
    (:`then`
      (set `/Game/Player/BP_Player.IsAtCauldron` true _asbp_player))
    (:`CastFailed`
      ;[1 1 1] Check that the item is an ingredient via BPI_INGREDIENTS and if so then stores which types have been added
      (bind _asbpi_ingredients (cast `/Game/Objects/Ingredients/BPI_Ingredients` OtherActor))
      (bind _ingredienttype (`/Game/Objects/Ingredients/BPI_Ingredients.GetIngredientType` _asbpi_ingredients))
      (`KismetArrayLibrary.Array_Add` (`self.AddedIngredients`) _ingredienttype)
      (switch `/Game/Objects/Ingredients/E_IngredientType` _ingredienttype
        (:`NewEnumerator0`
          _)
        (:`NewEnumerator1`
          _)
        (:`NewEnumerator2`
          _)
        (:`NewEnumerator3`
          _)
        (:`NewEnumerator4`
          _)
        (:`NewEnumerator5`
          _)
        (:`NewEnumerator6`
          _)
        (:`NewEnumerator7`
          _)
        (:`NewEnumerator8`
          _)
        (:`NewEnumerator9`
          _)
        (:`NewEnumerator10`
          _)
        (:`NewEnumerator11`
          _))
      (`self.K2_DestroyActor` OtherActor)
      (`AddComponent|NODE_AddNiagaraComponent-0`)
      (`self.CheckAddedIngredients`))))

(event `Summon`
  ;[1 1 1] Summon the demon and reset added ingredients + stir bools
  (`KismetSystemLibrary.PrintString` "Summoning demon")
  (bind _outactors (`GameplayStatics.GetAllActorsOfClassWithTag` "/Game/Objects/BP_SummoningCircle.BP_SummoningCircle_C" "poop"))
  (`/Game/Objects/BP_SummoningCircle.Summon` _outactors)
  (`KismetArrayLibrary.Array_Clear` (`self.AddedIngredients`))
  (set `self.IsClockwiseStirred` false)
  (set `self.IsAnticlockwiseStirred` false))

(event `self.ReceiveBeginPlay`
  (bind _returnvalue (`|CreateWidget` "/Game/UI/P_Summon.P_Summon_C"))
  (set `self.AddIngredientsPrompt` _returnvalue)
  (`self.UpdateCurrentRecipe`))

(event `self.PromptBox.OnComponentBeginOverlap`
  (params (OverlappedComponent :type "PrimitiveComponent Object Reference") (OtherActor :type "Actor Object Reference") (OtherComp :type "PrimitiveComponent Object Reference") (OtherBodyIndex :type Integer) (bFromSweep :type Boolean) (SweepResult :type "HitResult Structure (by ref)"))
  ;[1 1 1] Interact Prompt
  (if (== OtherActor (`GameplayStatics.GetPlayerCharacter` 0))
    (`UserWidget.AddToViewport` (`self.AddIngredientsPrompt`) 0)
    (if (`self.isDirty`) :!label _label
      (bind _returnvalue (`|CreateWidget` "/Game/UI/P_CleanCauldron.P_CleanCauldron_C"))
      (bind _output_get (set `self.CleanCauldronWidget` _returnvalue))
      (`UserWidget.AddToViewport` _output_get 0))))

(event `self.PromptBox.OnComponentEndOverlap`
  (params (OverlappedComponent :type "PrimitiveComponent Object Reference") (OtherActor :type "Actor Object Reference") (OtherComp :type "PrimitiveComponent Object Reference") (OtherBodyIndex :type Integer))
  ;[1 1 1] Interact Prompt
  (if (== (`GameplayStatics.GetPlayerCharacter` 0) OtherActor)
    (`Widget.RemoveFromParent` (`self.AddIngredientsPrompt`))
    (goto _label)))

(event `self.Sphere.OnComponentBeginOverlap`
  (params (OverlappedComponent :type "PrimitiveComponent Object Reference") (OtherActor :type "Actor Object Reference") (OtherComp :type "PrimitiveComponent Object Reference") (OtherBodyIndex :type Integer) (bFromSweep :type Boolean) (SweepResult :type "HitResult Structure (by ref)"))
  (`SceneComponent.SetVisibility` (`self.Widget`) true false))

(event `self.Sphere.OnComponentEndOverlap`
  (params (OverlappedComponent :type "PrimitiveComponent Object Reference") (OtherActor :type "Actor Object Reference") (OtherComp :type "PrimitiveComponent Object Reference") (OtherBodyIndex :type Integer))
  (`SceneComponent.SetVisibility` (`self.Widget`) false false))

(event `CleanCauldron`
  ;[1 1 1] Clean Cauldron
  (if (`self.isDirty`)
    (bind _asbp_player (cast `/Game/Player/BP_Player` (`GameplayStatics.GetPlayerCharacter` 0)))
    (if (`/Game/Player/BP_Player.IsAtCauldron` _asbp_player)
      (`AddComponent|NODE_AddNiagaraComponent-3`)
      (set `self.isDirty` false)
      (`PrimitiveComponent.SetMaterial` (`self.StaticMesh`) 0 "/Game/Materials/MI_Props_Cauldron.MI_Props_Cauldron")
      (bind _asfinn_game_instance (cast `/Game/Blueprints/FinnGameInstance` (`GameplayStatics.GetGameInstance`)))
      (set `/Game/Blueprints/FinnGameInstance.IsRecipeCorrect` false _asfinn_game_instance)
      (`self.UpdateCurrentRecipe`)
      (`WidgetLayoutLibrary.RemoveAllWidgets`)
      (`KismetSystemLibrary.PrintString` "Cleaned"))))

(event `UpdateCurrentRecipe`
  (bind _returnvalue (`self.GetTransform`))
  ;[1 1 1] Updates the current recipe
  (bind _asfinn_game_instance (cast `/Game/Blueprints/FinnGameInstance` (`GameplayStatics.GetGameInstance`)))
  (switch `/Game/Recipes/ERecipes` (`/Game/Blueprints/FinnGameInstance.CurrentRecipe` _asfinn_game_instance)
    (:`NewEnumerator0`
      (bind _returnvalue_2 (`|SpawnActorFromClass` "/Game/Recipes/BP_Recipe_1.BP_Recipe_1_C" _returnvalue "Undefined" "MultiplyWithRoot" null null))
      (bind _output_get (set `self.Recipe` _returnvalue_2))
      (set `/Game/Blueprints/FinnGameInstance.CurrentRecipeActor` _output_get _asfinn_game_instance))
    (:`NewEnumerator1`
      (bind _returnvalue_3 (`|SpawnActorFromClass` "/Game/Recipes/BP_Recipe_2.BP_Recipe_2_C" _returnvalue "Undefined" "MultiplyWithRoot" null null))
      (bind _output_get_2 (set `self.Recipe` _returnvalue_3))
      (set `/Game/Blueprints/FinnGameInstance.CurrentRecipeActor` _output_get_2 _asfinn_game_instance))
    (:`NewEnumerator2`
      (bind _returnvalue_4 (`|SpawnActorFromClass` "/Game/Recipes/BP_Recipe_3.BP_Recipe_3_C" _returnvalue "Undefined" "MultiplyWithRoot" null null))
      (bind _output_get_3 (set `self.Recipe` _returnvalue_4))
      (set `/Game/Blueprints/FinnGameInstance.CurrentRecipeActor` _output_get_3 _asfinn_game_instance))
    (:`NewEnumerator3`
      (bind _returnvalue_5 (`|SpawnActorFromClass` "/Game/Recipes/BP_Recipe_4.BP_Recipe_4_C" _returnvalue "Undefined" "MultiplyWithRoot" null null))
      (bind _output_get_4 (set `self.Recipe` _returnvalue_5))
      (set `/Game/Blueprints/FinnGameInstance.CurrentRecipeActor` _output_get_4 _asfinn_game_instance))
    (:`NewEnumerator4`
      (bind _returnvalue_6 (`|SpawnActorFromClass` "/Game/Recipes/BP_Recipe_5.BP_Recipe_5_C" _returnvalue "Undefined" "MultiplyWithRoot" null null))
      (bind _output_get_5 (set `self.Recipe` _returnvalue_6))
      (set `/Game/Blueprints/FinnGameInstance.CurrentRecipeActor` _output_get_5 _asfinn_game_instance))
    (:`NewEnumerator5`
      (bind _returnvalue_7 (`|SpawnActorFromClass` "/Game/Recipes/BP_Recipe_6.BP_Recipe_6_C" _returnvalue "Undefined" "MultiplyWithRoot" null null))
      (bind _output_get_6 (set `self.Recipe` _returnvalue_7))
      (set `/Game/Blueprints/FinnGameInstance.CurrentRecipeActor` _output_get_6 _asfinn_game_instance))
    (:`NewEnumerator6`
      (bind _returnvalue_8 (`|SpawnActorFromClass` "/Game/Recipes/BP_Recipe_7.BP_Recipe_7_C" _returnvalue "Undefined" "MultiplyWithRoot" null null))
      (bind _output_get_7 (set `self.Recipe` _returnvalue_8))
      (set `/Game/Blueprints/FinnGameInstance.CurrentRecipeActor` _output_get_7 _asfinn_game_instance))
    (:`NewEnumerator7`
      (bind _returnvalue_9 (`|SpawnActorFromClass` "/Game/Recipes/BP_Recipe_8.BP_Recipe_8_C" _returnvalue "Undefined" "MultiplyWithRoot" null null))
      (bind _output_get_8 (set `self.Recipe` _returnvalue_9))
      (set `/Game/Blueprints/FinnGameInstance.CurrentRecipeActor` _output_get_8 _asfinn_game_instance))
    (:`NewEnumerator8`
      (bind _returnvalue_10 (`|SpawnActorFromClass` "/Game/Recipes/BP_Recipe_9.BP_Recipe_9_C" _returnvalue "Undefined" "MultiplyWithRoot" null null))
      (bind _output_get_9 (set `self.Recipe` _returnvalue_10))
      (set `/Game/Blueprints/FinnGameInstance.CurrentRecipeActor` _output_get_9 _asfinn_game_instance))
    (:`NewEnumerator9`
      (bind _returnvalue_11 (`|SpawnActorFromClass` "/Game/Recipes/BP_Recipe_10.BP_Recipe_10_C" _returnvalue "Undefined" "MultiplyWithRoot" null null))
      (bind _output_get_10 (set `self.Recipe` _returnvalue_11))
      (set `/Game/Blueprints/FinnGameInstance.CurrentRecipeActor` _output_get_10 _asfinn_game_instance)))
  (bind _asfinn_game_instance_2 (cast `/Game/Blueprints/FinnGameInstance` (`GameplayStatics.GetGameInstance`)))
  (set `/Game/Blueprints/FinnGameInstance.IsRecipeCorrect` false _asfinn_game_instance_2)
  (set `/Game/Blueprints/FinnGameInstance.CurrentRecipeActor` (`self.Recipe`) _asfinn_game_instance_2)
  (`self.UpdateRequiredIngredients`))

(event `UpdateRequiredIngredients`
  (bind _recipe (`self.Recipe`))
  ;[1 1 1] Update the current required ingredients based on current recipe
  (bind _asfinn_game_instance (cast `/Game/Blueprints/FinnGameInstance` (`GameplayStatics.GetGameInstance`)))
  (`/Game/Blueprints/FinnGameInstance.UpdateMoonState` _asfinn_game_instance)
  (bind _ingredient_1 (message `/Game/Recipes/BPI_RecipeFunctions.GetIngredient1` _recipe))
  (bind _output_get (set `self.Required_Ingredient_1` _ingredient_1))
  (bind _ingredient_2 (message `/Game/Recipes/BPI_RecipeFunctions.GetIngredient2` _recipe))
  (bind _output_get_2 (set `self.Required_Ingredient_2` _ingredient_2))
  (bind _ingredient_3 (message `/Game/Recipes/BPI_RecipeFunctions.GetIngredient3` _recipe))
  (bind _output_get_3 (set `self.Required_Ingredient_3` _ingredient_3))
  (`KismetSystemLibrary.PrintString` (`|GetEnumeratorNameAsString` _output_get))
  (`KismetSystemLibrary.PrintString` (`|GetEnumeratorNameAsString` _output_get_2))
  (`KismetSystemLibrary.PrintString` (`|GetEnumeratorNameAsString` _output_get_3)))

(event `CheckAddedIngredients`
  (if (== (`KismetArrayLibrary.Array_Length` (`self.AddedIngredients`)) 3)
    (if (== (`self.Required_Ingredient_1`) (`|GetArrayItem` (`self.AddedIngredients`)))
      (if (== (`self.Required_Ingredient_2`) (`|GetArrayItem` (`self.AddedIngredients`) 1))
        (if (== (`self.Required_Ingredient_3`) (`|GetArrayItem` (`self.AddedIngredients`) 2))
          (if (`self.isDirty`)
            (`GameplayStatics.PlaySound2D` "/Game/Sounds/devil_cauldron_not_clean_fail.devil_cauldron_not_clean_fail" 1.0 1.0 0.0 null null)
            (else
              (bind _asfinn_game_instance (cast `/Game/Blueprints/FinnGameInstance` (`GameplayStatics.GetGameInstance`)))
              (set `/Game/Blueprints/FinnGameInstance.IsRecipeCorrect` true _asfinn_game_instance)))
          (else
            (`KismetSystemLibrary.PrintString` "third ingredient wrong")
            ;[1 1 1] Make Cauldron Dirty and recipe incorrect
            (`KismetSystemLibrary.PrintString` "RECIPE WRONG!" :!label _label_2)
            (bind _asfinn_game_instance_2 (cast `/Game/Blueprints/FinnGameInstance` (`GameplayStatics.GetGameInstance`)))
            (set `/Game/Blueprints/FinnGameInstance.IsRecipeCorrect` false _asfinn_game_instance_2)))
        (else
          (`KismetSystemLibrary.PrintString` "second ingredient wrong")
          (goto _label_2)))
      (else
        (`KismetSystemLibrary.PrintString` "first ingredient wrong")
        (goto _label_2)))
    (else
      ;[1 1 1] Check if more than 3 ingredients added
      (if (> (`KismetArrayLibrary.Array_Length` (`self.AddedIngredients`)) 3)
        (goto _label_2)))))

(event `SpawnGoopeyDemon`
  ;[1 1 1] Summon a goopey gooey dead demon
  (set `self.isDirty` true)
  (`PrimitiveComponent.SetMaterial` (`self.StaticMesh`) 0 "/Game/Materials/MI_WallDmg_Inst.MI_WallDmg_Inst")
  (bind _asbp_player (cast `/Game/Player/BP_Player` (`GameplayStatics.GetPlayerCharacter` 0)))
  (`/Game/Player/BP_Player.DEATH!` _asbp_player)
  (`GameplayStatics.PlaySound2D` "/Game/Sounds/deaddemonreaction.deaddemonreaction" 1.0 1.0 0.0 null null))

(event `SuccessfulRecipe`
  ;[1 1 1] Successful recipe
  (`AddComponent|NODE_AddNiagaraComponent-4`)
  (`KismetArrayLibrary.Array_Clear` (`self.AddedIngredients`))
  (`KismetSystemLibrary.PrintString` "recipe successful, array cleared")
  (set `self.isDirty` true)
  (`PrimitiveComponent.SetMaterial` (`self.StaticMesh`) 0 "/Game/Materials/MI_WallDmg_Inst.MI_WallDmg_Inst")
  (`GameplayStatics.PlaySound2D` "/Game/Sounds/devil_laugh_summon_success.devil_laugh_summon_success" 1.0 1.0 0.0 null null)
  (`KismetSystemLibrary.Delay` 8.0)
  (bind _asfinn_game_instance (cast `/Game/Blueprints/FinnGameInstance` (`GameplayStatics.GetGameInstance`)))
  (`/Game/Blueprints/FinnGameInstance.ProcessCorrectRecipe` _asfinn_game_instance))

(fn `UserConstructionScript`)