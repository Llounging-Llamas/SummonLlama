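; BP_Knife is an interactable knife pickup that the player collects.
; On Interact, it casts the first player character to BP_Player, passes its static mesh and itself as the picked-up item, and sets HasKnife.
; It then waits a very short delay, destroys itself and prints a pickup message, so the PickedUpItem reference points to a destroyed actor.
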(event `/Game/Objects/BPI_Interact.Interact`
  ;[1 1 1] Pick up the spoon
  (bind _asbp_player (cast `/Game/Player/BP_Player` (`GameplayStatics.GetPlayerCharacter` 0)))
  (set `/Game/Player/BP_Player.PickedUpItemMesh` (`StaticMeshComponent.StaticMesh` (`self.StaticMesh`)) _asbp_player)
  (set `/Game/Player/BP_Player.HasKnife` true _asbp_player)
  (set `/Game/Player/BP_Player.PickedUpItem` self _asbp_player)
  (`KismetSystemLibrary.Delay` 0.01)
  (`self.K2_DestroyActor`)
  (`KismetSystemLibrary.PrintString` "Knife Picked Up"))

(fn `UserConstructionScript`)