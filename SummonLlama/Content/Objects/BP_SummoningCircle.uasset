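; Summoning circle actor that spawns one of three summon classes when its Summon event is called.
; The event casts the game instance to FinnGameInstance and switches on its SummonType to pick Summon1, Summon2 or Summon3.
; The chosen actor spawns a fixed height above the circle's root, followed by a debug print.
; A disconnected spawn node with no class remains unused.
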(event `Summon`
  (bind (_returnvalue_x _returnvalue_y _returnvalue_z) (`KismetMathLibrary.BreakVector` (`SceneComponent.K2_GetComponentLocation` (`self.DefaultSceneRoot`))))
  (bind _returnvalue (`KismetMathLibrary.MakeTransform` (`KismetMathLibrary.MakeVector` _returnvalue_x _returnvalue_y (+ _returnvalue_z 200.0))))
  (bind _asfinn_game_instance (cast `/Game/Blueprints/FinnGameInstance` (`GameplayStatics.GetGameInstance`)))
  (switch `int` (`/Game/Blueprints/FinnGameInstance.SummonType` _asfinn_game_instance)
    (:`1`
      (`|SpawnActorFromClass` "/Game/Objects/Summon1.Summon1_C" _returnvalue "Undefined" "MultiplyWithRoot" null null))
    (:`2`
      (`|SpawnActorFromClass` "/Game/Objects/Summon2.Summon2_C" _returnvalue "Undefined" "MultiplyWithRoot" null null))
    (:`3`
      (`|SpawnActorFromClass` "/Game/Objects/Summon3.Summon3_C" _returnvalue "Undefined" "MultiplyWithRoot" null null)))
  (`KismetSystemLibrary.PrintString` "SUMMON SPAWN"))

(fn `UserConstructionScript`)