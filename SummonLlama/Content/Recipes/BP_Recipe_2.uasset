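; BP_Recipe_2 is a recipe Blueprint that holds the data for one recipe: its name, three ingredients and an actor to spawn.
; Getter functions return each of these variables.
; It has no runtime logic of its own: the event stubs are disabled and the construction script is empty.
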(fn `GetActorToSpawn`
  (returns (`Actor To Spawn` :type "Actor Class Reference"))
  (return (`self.ActorToSpawn`)))

(fn `GetIngredient1`
  (returns (`Ingredient 1` :type "/Game/Objects/Ingredients/E_IngredientType Enum"))
  (return (`self.Ingredient_1`)))

(fn `GetIngredient2`
  (returns (`Ingredient 2` :type "/Game/Objects/Ingredients/E_IngredientType Enum"))
  (return (`self.Ingredient_2`)))

(fn `GetIngredient3`
  (returns (`Ingredient 3` :type "/Game/Objects/Ingredients/E_IngredientType Enum"))
  (return (`self.Ingredient_3`)))

(fn `GetRecipeName`
  (returns (RecipeName :type String))
  (return (`self.RecipeName`)))

(fn `UserConstructionScript`)