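; Recipe actor that holds a recipe name, three ingredient slots and the actor to spawn, exposed through getter functions.
; Each ingredient getter reads IsMoonVisible from FinnGameInstance and returns the stored ingredient normally, or a fixed substitute with a different item and preparation state when the moon is visible.
; The substitution table is duplicated identically in all three getters, and the event graph and construction script contain no logic.
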(fn `GetActorToSpawn`
  (returns (`Actor To Spawn` :type "Actor Class Reference"))
  (return (`self.ActorToSpawn`)))

(fn `GetIngredient1`
  (returns (`Ingredient 1` :type "/Game/Objects/Ingredients/E_IngredientType Enum"))
  (bind _asfinn_game_instance (cast `/Game/Blueprints/FinnGameInstance` (`GameplayStatics.GetGameInstance`)))
  (switch `/Game/Objects/Ingredients/E_IngredientType` (`self.Ingredient_1`)
    (:`NewEnumerator0`
      (bind _ismoonvisible (`/Game/Blueprints/FinnGameInstance.IsMoonVisible` _asfinn_game_instance))
      (if _ismoonvisible
        (return "NewEnumerator11")
        (else
          (return "NewEnumerator0"))))
    (:`NewEnumerator1`
      (if _ismoonvisible
        (return "NewEnumerator9")
        (else
          (return "NewEnumerator1"))))
    (:`NewEnumerator2`
      (if _ismoonvisible
        (return "NewEnumerator10")
        (else
          (return "NewEnumerator2"))))
    (:`NewEnumerator3`
      (if _ismoonvisible
        (return "NewEnumerator8")
        (else
          (return "NewEnumerator3"))))
    (:`NewEnumerator4`
      (if _ismoonvisible
        (return "NewEnumerator6")
        (else
          (return "NewEnumerator4"))))
    (:`NewEnumerator5`
      (if _ismoonvisible
        (return "NewEnumerator7")
        (else
          (return "NewEnumerator5"))))
    (:`NewEnumerator6`
      (if _ismoonvisible
        (return "NewEnumerator2")
        (else
          (return "NewEnumerator6"))))
    (:`NewEnumerator7`
      (if _ismoonvisible
        (return "NewEnumerator0")
        (else
          (return "NewEnumerator7"))))
    (:`NewEnumerator8`
      (if _ismoonvisible
        (return "NewEnumerator1")
        (else
          (return "NewEnumerator8"))))
    (:`NewEnumerator9`
      (if _ismoonvisible
        (return "NewEnumerator5")
        (else
          (return "NewEnumerator9"))))
    (:`NewEnumerator10`
      (if _ismoonvisible
        (return "NewEnumerator3")
        (else
          (return "NewEnumerator10"))))
    (:`NewEnumerator11`
      (if _ismoonvisible
        (return "NewEnumerator4")
        (else
          (return "NewEnumerator11"))))))

(fn `GetIngredient2`
  (returns (`Ingredient 2` :type "/Game/Objects/Ingredients/E_IngredientType Enum"))
  (bind _asfinn_game_instance (cast `/Game/Blueprints/FinnGameInstance` (`GameplayStatics.GetGameInstance`)))
  (switch `/Game/Objects/Ingredients/E_IngredientType` (`self.Ingredient_2`)
    (:`NewEnumerator0`
      (bind _ismoonvisible (`/Game/Blueprints/FinnGameInstance.IsMoonVisible` _asfinn_game_instance))
      (if _ismoonvisible
        (return "NewEnumerator11")
        (else
          (return "NewEnumerator0"))))
    (:`NewEnumerator1`
      (if _ismoonvisible
        (return "NewEnumerator9")
        (else
          (return "NewEnumerator1"))))
    (:`NewEnumerator2`
      (if _ismoonvisible
        (return "NewEnumerator10")
        (else
          (return "NewEnumerator2"))))
    (:`NewEnumerator3`
      (if _ismoonvisible
        (return "NewEnumerator8")
        (else
          (return "NewEnumerator3"))))
    (:`NewEnumerator4`
      (if _ismoonvisible
        (return "NewEnumerator6")
        (else
          (return "NewEnumerator4"))))
    (:`NewEnumerator5`
      (if _ismoonvisible
        (return "NewEnumerator7")
        (else
          (return "NewEnumerator5"))))
    (:`NewEnumerator6`
      (if _ismoonvisible
        (return "NewEnumerator2")
        (else
          (return "NewEnumerator6"))))
    (:`NewEnumerator7`
      (if _ismoonvisible
        (return "NewEnumerator0")
        (else
          (return "NewEnumerator7"))))
    (:`NewEnumerator8`
      (if _ismoonvisible
        (return "NewEnumerator1")
        (else
          (return "NewEnumerator8"))))
    (:`NewEnumerator9`
      (if _ismoonvisible
        (return "NewEnumerator5")
        (else
          (return "NewEnumerator9"))))
    (:`NewEnumerator10`
      (if _ismoonvisible
        (return "NewEnumerator3")
        (else
          (return "NewEnumerator10"))))
    (:`NewEnumerator11`
      (if _ismoonvisible
        (return "NewEnumerator4")
        (else
          (return "NewEnumerator11"))))))

(fn `GetIngredient3`
  (returns (`Ingredient 3` :type "/Game/Objects/Ingredients/E_IngredientType Enum"))
  (bind _asfinn_game_instance (cast `/Game/Blueprints/FinnGameInstance` (`GameplayStatics.GetGameInstance`)))
  (switch `/Game/Objects/Ingredients/E_IngredientType` (`self.Ingredient_3`)
    (:`NewEnumerator0`
      (bind _ismoonvisible (`/Game/Blueprints/FinnGameInstance.IsMoonVisible` _asfinn_game_instance))
      (if _ismoonvisible
        (return "NewEnumerator11")
        (else
          (return "NewEnumerator0"))))
    (:`NewEnumerator1`
      (if _ismoonvisible
        (return "NewEnumerator9")
        (else
          (return "NewEnumerator1"))))
    (:`NewEnumerator2`
      (if _ismoonvisible
        (return "NewEnumerator10")
        (else
          (return "NewEnumerator2"))))
    (:`NewEnumerator3`
      (if _ismoonvisible
        (return "NewEnumerator8")
        (else
          (return "NewEnumerator3"))))
    (:`NewEnumerator4`
      (if _ismoonvisible
        (return "NewEnumerator6")
        (else
          (return "NewEnumerator4"))))
    (:`NewEnumerator5`
      (if _ismoonvisible
        (return "NewEnumerator7")
        (else
          (return "NewEnumerator5"))))
    (:`NewEnumerator6`
      (if _ismoonvisible
        (return "NewEnumerator2")
        (else
          (return "NewEnumerator6"))))
    (:`NewEnumerator7`
      (if _ismoonvisible
        (return "NewEnumerator0")
        (else
          (return "NewEnumerator7"))))
    (:`NewEnumerator8`
      (if _ismoonvisible
        (return "NewEnumerator1")
        (else
          (return "NewEnumerator8"))))
    (:`NewEnumerator9`
      (if _ismoonvisible
        (return "NewEnumerator5")
        (else
          (return "NewEnumerator9"))))
    (:`NewEnumerator10`
      (if _ismoonvisible
        (return "NewEnumerator3")
        (else
          (return "NewEnumerator10"))))
    (:`NewEnumerator11`
      (if _ismoonvisible
        (return "NewEnumerator4")
        (else
          (return "NewEnumerator11"))))))

(fn `GetRecipeName`
  (returns (RecipeName :type String))
  (return (`self.RecipeName`)))

(fn `UserConstructionScript`)